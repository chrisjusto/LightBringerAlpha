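; AI controller for a BasePlayer_BP combat fighter that picks and performs moves against its Enemy.
; Each Tick it compares both fighters' StateMachine states, attack-snap ranges and random rolls to queue an action in NextActionQue, or saves follow-up attacks mid-swing.
; Queued actions fire through pawn calls when clear, with delayed get-ups after knockdowns.
; An older flag-based decision tree and the timeline feeding the look-at rotation gate are disconnected.
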(event `self.ReceiveBeginPlay`
  (bind _asbase_player_bp (cast `/Game/Blueprints/CharacterBP/SECONDdRAFTcHARACTER/BasePlayer_BP` (`self.K2_GetPawn`)))
  (set `self.User` _asbase_player_bp)
  (`self.setrotation`))

(event `setrotation`
  (bind _user (`self.User`))
  (bind _enemy (`/Game/Blueprints/CharacterBP/SECONDdRAFTcHARACTER/BasePlayer_BP.Enemy` _user))
  ;[1 1 1] always look at player
  (`/Engine/EditorBlueprintResources/StandardMacros.Gate` true :!via `Toggle`
    (:`Exit`
      (`/Engine/EditorBlueprintResources/StandardMacros.IsValid` _user
        (:`Is Valid`
          (`/Engine/EditorBlueprintResources/StandardMacros.IsValid` _enemy
            (:`Is Valid`
              (if (not (`/Game/Blueprints/CharacterBP/SECONDdRAFTcHARACTER/BasePlayer_BP.hitFloor` _user))
                (`self.K2_SetActorRotation` _user (`KismetMathLibrary.MakeRotator` (.roll (`KismetMathLibrary.FindLookAtRotation` (`self.K2_GetActorLocation` _user) (`self.K2_GetActorLocation` _enemy))) 0.0 (.yaw (`KismetMathLibrary.FindLookAtRotation` (`self.K2_GetActorLocation` _user) (`self.K2_GetActorLocation` _enemy)))) false)))))))))

(event `self.ReceiveTick`
  (params (DeltaSeconds :type "Float (single-precision)"))
  (bind _user (`self.User`))
  (bind _user_2 (`self.User`))
  (bind _user_3 (`self.User`))
  (bind _user_4 (`self.User`))
  (bind _user_5 (`self.User`))
  (bind _user_6 (`self.User`))
  (bind _user_7 (`self.User`))
  (bind _user_8 (`self.User`))
  (bind _user_9 (`self.User`))
  (bind _user_10 (`self.User`))
  (bind _user_11 (`self.User`))
  (bind _user_12 (`self.User`))
  (bind _user_13 (`self.User`))
  (bind _statemachine (`/Game/Blueprints/CharacterBP/SECONDdRAFTcHARACTER/BasePlayer_BP.StateMachine` _user_3))
  (bind _canlightsnap_ (`/Game/Blueprints/CharacterBP/SECONDdRAFTcHARACTER/BasePlayer_BP.canLightSnap?` _user_5))
  (bind _enemy (`/Game/Blueprints/CharacterBP/SECONDdRAFTcHARACTER/BasePlayer_BP.Enemy` _user_12))
  (bind _canheavysnap_ (`/Game/Blueprints/CharacterBP/SECONDdRAFTcHARACTER/BasePlayer_BP.canHeavySnap?` _user_12))
  (bind _canlightsnap__2 (`/Game/Blueprints/CharacterBP/SECONDdRAFTcHARACTER/BasePlayer_BP.canLightSnap?` _user_12))
  (bind _statemachine_2 (`/Game/Blueprints/CharacterBP/SECONDdRAFTcHARACTER/BasePlayer_BP.StateMachine` (`/Game/Blueprints/CharacterBP/SECONDdRAFTcHARACTER/BasePlayer_BP.Enemy` _user_4)))
  ;[1 1 1] BothPartiesAreValid
  (`/Engine/EditorBlueprintResources/StandardMacros.IsValid` _user_8
    (:`Is Valid`
      (`/Engine/EditorBlueprintResources/StandardMacros.IsValid` (`/Game/Blueprints/CharacterBP/SECONDdRAFTcHARACTER/BasePlayer_BP.Enemy` _user_8)
        (:`Is Valid`
          ;[1 0 0.1541] followUp Logic and Actions
          (if (`|EnumEquality` (`/Game/Blueprints/CharacterBP/SECONDdRAFTcHARACTER/BasePlayer_BP.StateMachine` (`/Game/Blueprints/CharacterBP/SECONDdRAFTcHARACTER/BasePlayer_BP.Enemy` _user_10)) "NewEnumerator12")
            (set `self.nextActionQue` "NewEnumerator1")
            (`/Game/Blueprints/CharacterBP/SECONDdRAFTcHARACTER/BasePlayer_BP.CancelBlock` _user_10)
            (else
              ;;[1 1 1] checks if next action is cued
              (if (`|EnumEquality` (`self.nextActionQue`) "NewEnumerator0")
                ;;[1 1 1] check if user is in action
                (if (`|EnumEquality` (`/Game/Blueprints/CharacterBP/SECONDdRAFTcHARACTER/BasePlayer_BP.StateMachine` (`self.User`)) "NewEnumerator0")
                  ;[1 1 1] Response to players Actions
                  ;;[1 1 1] check if opponent is IDLE
                  (if (`|EnumEquality` _statemachine_2 "NewEnumerator0")
                    ;[1 1 1] AI_IdleFunctions
                    (if (`self.isClear` (`self.User`))
                      (if (`/Game/Blueprints/CharacterBP/SECONDdRAFTcHARACTER/BasePlayer_BP.canHeavySnap?` _user_13)
                        (set `self.nextActionQue` "NewEnumerator2")
                        (elif (`/Game/Blueprints/CharacterBP/SECONDdRAFTcHARACTER/BasePlayer_BP.canLightSnap?` _user_13)
                          (switch `int` (`KismetMathLibrary.RandomIntegerInRange` 0 1)
                            (:`0`
                              (set `self.nextActionQue` "NewEnumerator1"))
                            (:`1`
                              (set `/Game/Blueprints/CharacterBP/SECONDdRAFTcHARACTER/BasePlayer_BP.DashInput` "NewEnumerator0" (`self.User`))
                              (set `self.nextActionQue` "NewEnumerator3")))
                          (elif (not (`NavMovementComponent.IsFalling` (`Character.CharacterMovement` _user_13)))
                            (switch `int` (`KismetMathLibrary.RandomIntegerInRange` 0 8)
                              (:`0`
                                (set `/Game/Blueprints/CharacterBP/SECONDdRAFTcHARACTER/BasePlayer_BP.DashInput` "NewEnumerator0" (`self.User`) :!label _label)
                                (set `self.nextActionQue` "NewEnumerator3"))
                              (:`1`
                                (set `/Game/Blueprints/CharacterBP/SECONDdRAFTcHARACTER/BasePlayer_BP.DashInput` "NewEnumerator1" (`self.User`))
                                (set `self.nextActionQue` "NewEnumerator3"))
                              (:`2`
                                (set `/Game/Blueprints/CharacterBP/SECONDdRAFTcHARACTER/BasePlayer_BP.DashInput` "NewEnumerator2" (`self.User`))
                                (set `self.nextActionQue` "NewEnumerator3"))
                              (:`3`
                                (set `/Game/Blueprints/CharacterBP/SECONDdRAFTcHARACTER/BasePlayer_BP.DashInput` "NewEnumerator3" (`self.User`))
                                (set `self.nextActionQue` "NewEnumerator3"))
                              (:`4`
                                (set `self.nextActionQue` "NewEnumerator6"))
                              (:`5`
                                (set `self.nextActionQue` "NewEnumerator10")
                                (`AITask_MoveTo.AIMoveTo` null (`self.K2_GetActorLocation` (`/Game/Blueprints/CharacterBP/SECONDdRAFTcHARACTER/BasePlayer_BP.Enemy` (`self.User`))) null
                                  (:`OnRequestFailed`
                                    (set `self.nextActionQue` "NewEnumerator0"))
                                  (:`OnMoveFinished`
                                    (set `self.nextActionQue` "NewEnumerator0"))))
                              (:`6`
                                (goto _label))
                              (:`7`
                                (goto _label))
                              (:`8`
                                (goto _label)))
                            (else
                              (set `self.nextActionQue` "NewEnumerator0"))))))
                    (else
                      ;;[1 1 1] setActions
                      (if (`self.isClear` _user_4)
                        (switch `/Game/Blueprints/enums/PlayerStates` _statemachine_2
                          (:`NewEnumerator1`
                            (if (`/Game/Blueprints/CharacterBP/SECONDdRAFTcHARACTER/BasePlayer_BP.canLightSnap?` _enemy)
                              (set `self.nextActionQue` "NewEnumerator5")
                              (elif (`/Game/Blueprints/CharacterBP/SECONDdRAFTcHARACTER/BasePlayer_BP.canLightSnap?` (`self.User`))
                                (set `self.nextActionQue` "NewEnumerator1"))))
                          (:`NewEnumerator2`
                            (if (`/Game/Blueprints/CharacterBP/SECONDdRAFTcHARACTER/BasePlayer_BP.canLightSnap?` _user_12)
                              (set `self.nextActionQue` "NewEnumerator1")
                              (else
                                (switch `int` (`KismetMathLibrary.RandomIntegerInRange` 0 1)
                                  (:`0`
                                    (set `/Game/Blueprints/CharacterBP/SECONDdRAFTcHARACTER/BasePlayer_BP.DashInput` "NewEnumerator2" _user_12)
                                    (set `self.nextActionQue` "NewEnumerator3"))
                                  (:`1`
                                    (set `/Game/Blueprints/CharacterBP/SECONDdRAFTcHARACTER/BasePlayer_BP.DashInput` "NewEnumerator3" _user_12)
                                    (set `self.nextActionQue` "NewEnumerator3"))))))
                          (:`NewEnumerator3`
                            (if _canheavysnap_
                              (set `self.nextActionQue` "NewEnumerator2" :!label _label_2)
                              (elif _canlightsnap__2
                                (set `self.nextActionQue` "NewEnumerator1" :!label _label_3)
                                (else
                                  (switch `/Game/Blueprints/enums/Input_Enums` (`/Game/Blueprints/CharacterBP/SECONDdRAFTcHARACTER/BasePlayer_BP.DashInput` _enemy)
                                    (:`NewEnumerator0`
                                      (set `/Game/Blueprints/CharacterBP/SECONDdRAFTcHARACTER/BasePlayer_BP.DashInput` "NewEnumerator1" _user_12)
                                      (set `self.nextActionQue` "NewEnumerator3"))
                                    (:`NewEnumerator1`
                                      (set `/Game/Blueprints/CharacterBP/SECONDdRAFTcHARACTER/BasePlayer_BP.DashInput` "NewEnumerator0" _user_12 :!label _label_4)
                                      (set `self.nextActionQue` "NewEnumerator3"))
                                    (:`NewEnumerator2`
                                      (goto _label_4))
                                    (:`NewEnumerator3`
                                      (goto _label_4)))))))
                          (:`NewEnumerator4`
                            (if _canheavysnap_
                              (goto _label_2)
                              (elif _canlightsnap__2
                                (goto _label_3)
                                (else
                                  (goto _label_4)))))
                          (:`NewEnumerator5`
                            (if _canheavysnap_
                              (goto _label_2)
                              (elif _canlightsnap__2
                                (goto _label_3)
                                (else
                                  (switch `int` (`KismetMathLibrary.RandomIntegerInRange` 0 2)
                                    (:`0`
                                      (set `self.nextActionQue` "NewEnumerator0"))
                                    (:`1`
                                      (set `/Game/Blueprints/CharacterBP/SECONDdRAFTcHARACTER/BasePlayer_BP.DashInput` "NewEnumerator0" _user_12)
                                      (set `self.nextActionQue` "NewEnumerator3"))
                                    (:`2`
                                      (set `self.nextActionQue` "NewEnumerator6")))))))
                          (:`NewEnumerator6`
                            (switch `int` (`KismetMathLibrary.RandomIntegerInRange` 0 2)
                              (:`0`
                                (set `self.nextActionQue` "NewEnumerator5"))
                              (:`1`
                                (set `/Game/Blueprints/CharacterBP/SECONDdRAFTcHARACTER/BasePlayer_BP.DashInput` "NewEnumerator2" _user_12)
                                (set `self.nextActionQue` "NewEnumerator3"))
                              (:`2`
                                (set `/Game/Blueprints/CharacterBP/SECONDdRAFTcHARACTER/BasePlayer_BP.DashInput` "NewEnumerator3" _user_12)
                                (set `self.nextActionQue` "NewEnumerator3"))))
                          (:`NewEnumerator7`
                            (if (`/Game/Blueprints/CharacterBP/SECONDdRAFTcHARACTER/BasePlayer_BP.canHeavySnap?` _user)
                              (set `self.nextActionQue` "NewEnumerator2")
                              (elif (`/Game/Blueprints/CharacterBP/SECONDdRAFTcHARACTER/BasePlayer_BP.canLightSnap?` _user)
                                (switch `int` (`KismetMathLibrary.RandomIntegerInRange` 0 1)
                                  (:`0`
                                    (set `/Game/Blueprints/CharacterBP/SECONDdRAFTcHARACTER/BasePlayer_BP.DashInput` "NewEnumerator0" _user)
                                    (set `self.nextActionQue` "NewEnumerator3"))
                                  (:`1`
                                    (set `self.nextActionQue` "NewEnumerator1")))
                                (else
                                  (set `/Game/Blueprints/CharacterBP/SECONDdRAFTcHARACTER/BasePlayer_BP.DashInput` "NewEnumerator0" _user)
                                  (set `self.nextActionQue` "NewEnumerator3")))))))))
                  (else
                    ;;[1 1 1] sets next action
                    (switch `/Game/Blueprints/enums/PlayerStates` (`/Game/Blueprints/CharacterBP/SECONDdRAFTcHARACTER/BasePlayer_BP.StateMachine` (`self.User`))
                      (:`NewEnumerator1`
                        (set `/Game/Blueprints/CharacterBP/SECONDdRAFTcHARACTER/BasePlayer_BP.saveLightAttack` true _user_7))
                      (:`NewEnumerator2`
                        (set `/Game/Blueprints/CharacterBP/SECONDdRAFTcHARACTER/BasePlayer_BP.saveHeavyAttack` true _user_7))
                      (:`NewEnumerator3`
                        (switch `/Game/Blueprints/enums/Input_Enums` (`/Game/Blueprints/CharacterBP/SECONDdRAFTcHARACTER/BasePlayer_BP.DashInput` _user_7)
                          (:`NewEnumerator0`
                            (if (`/Game/Blueprints/CharacterBP/SECONDdRAFTcHARACTER/BasePlayer_BP.canHeavySnap?` _user_5)
                              (set `self.nextActionQue` "NewEnumerator2")
                              (elif _canlightsnap_
                                (set `self.nextActionQue` "NewEnumerator1")
                                (else
                                  (set `/Game/Blueprints/CharacterBP/SECONDdRAFTcHARACTER/BasePlayer_BP.DashInput` "NewEnumerator0" _user_7)
                                  (set `self.nextActionQue` "NewEnumerator3")))))
                          (:`NewEnumerator1`
                            (if _canlightsnap_ :!label _label_5
                              (set `self.nextActionQue` "NewEnumerator1")
                              (else
                                (set `self.nextActionQue` "NewEnumerator0"))))
                          (:`NewEnumerator2`
                            (goto _label_5))
                          (:`NewEnumerator3`
                            (goto _label_5))))
                      (:`NewEnumerator4`
                        (set `/Game/Blueprints/CharacterBP/SECONDdRAFTcHARACTER/BasePlayer_BP.DashInput` "NewEnumerator1" _user_7)
                        (set `self.nextActionQue` "NewEnumerator3"))
                      (:`NewEnumerator5`
                        (switch `int` (`KismetMathLibrary.RandomIntegerInRange` 0 2)
                          (:`0`
                            (if (`/Game/Blueprints/CharacterBP/SECONDdRAFTcHARACTER/BasePlayer_BP.canLightSnap?` _user_2)
                              (set `self.nextActionQue` "NewEnumerator1")
                              (else
                                (set `/Game/Blueprints/CharacterBP/SECONDdRAFTcHARACTER/BasePlayer_BP.DashInput` "NewEnumerator0" _user_2)
                                (set `self.nextActionQue` "NewEnumerator3"))))
                          (:`1`
                            (set `/Game/Blueprints/CharacterBP/SECONDdRAFTcHARACTER/BasePlayer_BP.DashInput` "NewEnumerator3" _user_2)
                            (set `self.nextActionQue` "NewEnumerator3"))
                          (:`2`
                            (set `/Game/Blueprints/CharacterBP/SECONDdRAFTcHARACTER/BasePlayer_BP.DashInput` "NewEnumerator2" _user_2)
                            (set `self.nextActionQue` "NewEnumerator3"))))
                      (:`NewEnumerator6`
                        (if (`/Game/Blueprints/CharacterBP/SECONDdRAFTcHARACTER/BasePlayer_BP.canHeavySnap?` _user_7)
                          (set `self.nextActionQue` "NewEnumerator2")
                          (elif (`/Game/Blueprints/CharacterBP/SECONDdRAFTcHARACTER/BasePlayer_BP.canLightSnap?` _user_7)
                            (set `self.nextActionQue` "NewEnumerator1"))))
                      (:`NewEnumerator7`
                        (switch `int` (`KismetMathLibrary.RandomIntegerInRange` 0 3)
                          (:`0`
                            (set `self.nextActionQue` "NewEnumerator5"))
                          (:`1`
                            (set `self.nextActionQue` "NewEnumerator3")
                            (set `/Game/Blueprints/CharacterBP/SECONDdRAFTcHARACTER/BasePlayer_BP.DashInput` "NewEnumerator1" _user_6))
                          (:`2`
                            (set `self.nextActionQue` "NewEnumerator3")
                            (set `/Game/Blueprints/CharacterBP/SECONDdRAFTcHARACTER/BasePlayer_BP.DashInput` "NewEnumerator2" _user_6))
                          (:`3`
                            (set `self.nextActionQue` "NewEnumerator3")
                            (set `/Game/Blueprints/CharacterBP/SECONDdRAFTcHARACTER/BasePlayer_BP.DashInput` "NewEnumerator3" _user_6))))
                      (:`NewEnumerator11`
                        (`KismetSystemLibrary.Delay` (`KismetMathLibrary.RandomFloatInRange` 0.0 3.0))
                        (`/Game/Blueprints/CharacterBP/SECONDdRAFTcHARACTER/BasePlayer_BP.callGetUp` (`self.User`))
                        (set `self.nextActionQue` "NewEnumerator0")))))
                (elif (`|EnumEquality` _statemachine "NewEnumerator11")
                  (`KismetSystemLibrary.Delay` (`KismetMathLibrary.RandomFloatInRange` 0.0 3.0))
                  (`/Game/Blueprints/CharacterBP/SECONDdRAFTcHARACTER/BasePlayer_BP.callGetUp` _user_3)
                  (if (`/Game/Blueprints/CharacterBP/SECONDdRAFTcHARACTER/BasePlayer_BP.canHeavySnap?` _user_9)
                    (set `self.nextActionQue` "NewEnumerator2")
                    (elif (`/Game/Blueprints/CharacterBP/SECONDdRAFTcHARACTER/BasePlayer_BP.canLightSnap?` _user_9)
                      (set `self.nextActionQue` "NewEnumerator1")
                      (else
                        (set `/Game/Blueprints/CharacterBP/SECONDdRAFTcHARACTER/BasePlayer_BP.DashInput` "NewEnumerator1" _user_9)
                        (set `self.nextActionQue` "NewEnumerator3"))))
                  (elif (and (`|EnumEquality` (`/Game/Blueprints/CharacterBP/SECONDdRAFTcHARACTER/BasePlayer_BP.StateMachine` (`/Game/Blueprints/CharacterBP/SECONDdRAFTcHARACTER/BasePlayer_BP.Enemy` _user_3)) "NewEnumerator12") (`|EnumEquality` _statemachine "NewEnumerator1"))
                    ;;[1 1 1] Calls Next Action
                    (`/Game/Blueprints/CharacterBP/SECONDdRAFTcHARACTER/BasePlayer_BP.CancelBlock` _user_11)
                    (`/Game/Blueprints/CharacterBP/SECONDdRAFTcHARACTER/BasePlayer_BP.canLightAttack` _user_11 :!label _label_6)
                    (set `self.nextActionQue` "NewEnumerator0" :!label _label_7)
                    (elif (`self.isClear` _user_8)
                      (switch `/Game/Blueprints/enums/PlayerStates` (`self.nextActionQue`)
                        (:`NewEnumerator1`
                          (goto _label_6))
                        (:`NewEnumerator2`
                          (`/Game/Blueprints/CharacterBP/SECONDdRAFTcHARACTER/BasePlayer_BP.canHeavyAttack` _user_11)
                          (goto _label_7))
                        (:`NewEnumerator3`
                          (`/Game/Blueprints/CharacterBP/SECONDdRAFTcHARACTER/BasePlayer_BP.callDashAnimation` _user_11 (`/Game/Blueprints/CharacterBP/SECONDdRAFTcHARACTER/BasePlayer_BP.DashInput` _user_11))
                          (goto _label_7))
                        (:`NewEnumerator4`
                          (`/Game/Blueprints/CharacterBP/SECONDdRAFTcHARACTER/BasePlayer_BP.callHeal` _user_11)
                          (goto _label_7))
                        (:`NewEnumerator5`
                          (`/Game/Blueprints/CharacterBP/SECONDdRAFTcHARACTER/BasePlayer_BP.callGaurd` _user_11)
                          (goto _label_7))
                        (:`NewEnumerator6`
                          (`/Game/Blueprints/CharacterBP/SECONDdRAFTcHARACTER/BasePlayer_BP.callProjectile` _user_11)
                          (goto _label_7))))))))))))))

(fn `UserConstructionScript`)