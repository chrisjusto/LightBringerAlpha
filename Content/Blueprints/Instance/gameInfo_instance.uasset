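; Game instance that holds gameplay counters and reports them as analytics on player attacks, movement and combat.
; The Analytics event opens a session, records one attribute-tagged event per category, then ends the session.
; Play time is read from game time just before the combat event is recorded.
; Shutdown is empty, and the only Analytics call in this graph is disconnected, so nothing here triggers the report.
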(event `self.ReceiveShutdown`
  ;[1 1 1] Event Shutdown
)

(event `Analytics`
  ;[1 1 1] Metrics
  (`AnalyticsBlueprintLibrary.StartSession`)
  (`AnalyticsBlueprintLibrary.RecordEventWithAttributes` "Player Attacks" (`|MakeArray` (make `AnalyticsEventAttr` "Light Swing" (`KismetStringLibrary.Conv_IntToString` (`self.lightSwing`))) (make `AnalyticsEventAttr` "Light Hit" (`KismetStringLibrary.Conv_IntToString` (`self.lightHit`))) (make `AnalyticsEventAttr` "Light Blocked by Enemy" (`KismetStringLibrary.Conv_IntToString` (`self.lightBlockedByEnemy`))) (make `AnalyticsEventAttr` "Light Blocked by Player" (`KismetStringLibrary.Conv_IntToString` (`self.lightBlockedByPlayer`))) (make `AnalyticsEventAttr` "Light Combo Complete" (`KismetStringLibrary.Conv_IntToString` (`self.lightComboComplete`))) (make `AnalyticsEventAttr` "Heavy Swing" (`KismetStringLibrary.Conv_IntToString` (`self.heavySwing`))) (make `AnalyticsEventAttr` "Heavy Hit" (`KismetStringLibrary.Conv_IntToString` (`self.heavyHit`))) (make `AnalyticsEventAttr` "Heavy Blocked by Enemy" (`KismetStringLibrary.Conv_IntToString` (`self.heavyBlockedByEnemy`))) (make `AnalyticsEventAttr` "Heavy Blocked by Player" (`KismetStringLibrary.Conv_IntToString` (`self.heavyBlockedByPlayer`))) (make `AnalyticsEventAttr` "Heavy Combo Completed" (`KismetStringLibrary.Conv_IntToString` (`self.heavyComboCompleted`))) (make `AnalyticsEventAttr` "Projectile Fired" (`KismetStringLibrary.Conv_IntToString` (`self.projectilesFired`))) (make `AnalyticsEventAttr` "Projectile Hit" (`KismetStringLibrary.Conv_IntToString` (`self.projectilesHit`)))))
  (`AnalyticsBlueprintLibrary.RecordEventWithAttributes` "Movement" (`|MakeArray` (make `AnalyticsEventAttr` "Dash Snaps" (`KismetStringLibrary.Conv_IntToString` (`self.dashSnaps`))) (make `AnalyticsEventAttr` "Dashes" (`KismetStringLibrary.Conv_IntToString` (`self.dashes`))) (make `AnalyticsEventAttr` "Time Spent Floating" (`KismetStringLibrary.Conv_DoubleToString` (`self.timeSpentFloating`)))))
  (set `self.playTimer` (`GameplayStatics.GetTimeSeconds`))
  (`AnalyticsBlueprintLibrary.RecordEventWithAttributes` "Combat" (`|MakeArray` (make `AnalyticsEventAttr` "Health Healed" (`KismetStringLibrary.Conv_IntToString` (`self.healthHealed`))) (make `AnalyticsEventAttr` "Damage Received" (`KismetStringLibrary.Conv_IntToString` (`self.damageReceived`))) (make `AnalyticsEventAttr` "Damage Dealt" (`KismetStringLibrary.Conv_IntToString` (`self.damageDealt`))) (make `AnalyticsEventAttr` "Player Deaths" (`KismetStringLibrary.Conv_IntToString` (`self.playerDeaths`))) (make `AnalyticsEventAttr` "Enemy Deaths" (`KismetStringLibrary.Conv_IntToString` (`self.enemyDeaths`))) (make `AnalyticsEventAttr` "Fights Started" (`KismetStringLibrary.Conv_IntToString` (`self.fightsStarted`))) (make `AnalyticsEventAttr` "Play Timer" (`KismetStringLibrary.Conv_DoubleToString` (`self.playTimer`)))))
  (`AnalyticsBlueprintLibrary.EndSession`))