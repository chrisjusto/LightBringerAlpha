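; Metric listener that records combat statistics for player and enemy in the gameInfo_instance game instance.
; Add functions update per-side counters for attacks, dashes, damage, healing and deaths, plus fights started.
; BeginPlay finds both characters; Tick times zero-gravity floating and banks it once gravity returns.
; Projectile tracking only prints a fix-later message, and enemy light swings get reset to zero instead of counted.
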(event `self.ReceiveBeginPlay`
  ;[1 1 1] Event BeginPlay
  (set `self.gameInfo_ref` (`GameplayStatics.GetGameInstance`))
  (`self.FindPlayer`))

(event `self.ReceiveTick`
  (params (DeltaSeconds :type "Float (single-precision)"))
  ;[1 1 1] Event Tick
  (`self.calculateTimeSpentFloating` DeltaSeconds))

(event `FindPlayer`
  ;[1 1 1] Get player reference
  (bind _outactors (`GameplayStatics.GetAllActorsOfClass` "/Game/Blueprints/CharacterBP/bp_baseCharacter.bp_baseCharacter_C"))
  (for _array_element _outactors
    (if (`|EnumEquality` (`/Game/Blueprints/CharacterBP/bp_baseCharacter.character` _array_element) "NewEnumerator0")
      (set `self.playerRef` _array_element)
      (else
        (set `self.enemyRef` _array_element)))))

(fn `addDamageDealt`
  (params (`Damage Dealt` :type Integer) (Character :type "/Game/Blueprints/enums/Character_Enums Enum" :default "NewEnumerator0"))
  (bind _asgame_info_instance (cast `/Game/Blueprints/Instance/gameInfo_instance` (`self.gameInfo_ref`)))
  (if (`|EnumEquality` Character "NewEnumerator0")
    (set `/Game/Blueprints/Instance/gameInfo_instance.Player_damageDealt` (+ (`/Game/Blueprints/Instance/gameInfo_instance.Player_damageDealt` _asgame_info_instance) `Damage Dealt`) _asgame_info_instance)
    (else
      (set `/Game/Blueprints/Instance/gameInfo_instance.Enemy_damageDealt` (+ (`/Game/Blueprints/Instance/gameInfo_instance.Enemy_damageDealt` _asgame_info_instance) `Damage Dealt`) _asgame_info_instance))))

(fn `addDamageReceived`
  (params (`Damage Received` :type Integer) (Character :type "/Game/Blueprints/enums/Character_Enums Enum" :default "NewEnumerator0"))
  (bind _asgame_info_instance (cast `/Game/Blueprints/Instance/gameInfo_instance` (`self.gameInfo_ref`)))
  (if (`|EnumEquality` Character "NewEnumerator0")
    (set `/Game/Blueprints/Instance/gameInfo_instance.Player_damageReceived` (+ (`/Game/Blueprints/Instance/gameInfo_instance.Player_damageReceived` _asgame_info_instance) `Damage Received`) _asgame_info_instance)
    (else
      (set `/Game/Blueprints/Instance/gameInfo_instance.Enemy_damageReceived` (+ (`/Game/Blueprints/Instance/gameInfo_instance.Enemy_damageReceived` _asgame_info_instance) `Damage Received`) _asgame_info_instance))))

(fn `addDash`
  (params (Character :type "/Game/Blueprints/enums/Character_Enums Enum" :default "NewEnumerator0"))
  (bind _asgame_info_instance (cast `/Game/Blueprints/Instance/gameInfo_instance` (`self.gameInfo_ref`)))
  (if (`|EnumEquality` Character "NewEnumerator0")
    (bind _result (`/Engine/EditorBlueprintResources/StandardMacros.IncrementInt` (`/Game/Blueprints/Instance/gameInfo_instance.Player_dashes` _asgame_info_instance))
      (:`  `
        (set `/Game/Blueprints/Instance/gameInfo_instance.Player_dashes` _result _asgame_info_instance)))
    (else
      (bind _result_2 (`/Engine/EditorBlueprintResources/StandardMacros.IncrementInt` (`/Game/Blueprints/Instance/gameInfo_instance.Enemy_dashes` _asgame_info_instance))
        (:`  `
          (set `/Game/Blueprints/Instance/gameInfo_instance.Enemy_dashes` _result_2 _asgame_info_instance))))))

(fn `addDashSnap`
  (params (Character :type "/Game/Blueprints/enums/Character_Enums Enum" :default "NewEnumerator0"))
  (bind _asgame_info_instance (cast `/Game/Blueprints/Instance/gameInfo_instance` (`self.gameInfo_ref`)))
  (if (`|EnumEquality` Character "NewEnumerator0")
    (bind _result (`/Engine/EditorBlueprintResources/StandardMacros.IncrementInt` (`/Game/Blueprints/Instance/gameInfo_instance.Player_dashSnaps` _asgame_info_instance))
      (:`  `
        (set `/Game/Blueprints/Instance/gameInfo_instance.Player_dashSnaps` _result _asgame_info_instance)))
    (else
      (bind _result_2 (`/Engine/EditorBlueprintResources/StandardMacros.IncrementInt` (`/Game/Blueprints/Instance/gameInfo_instance.Enemy_dashSnaps` _asgame_info_instance))
        (:`  `
          (set `/Game/Blueprints/Instance/gameInfo_instance.Enemy_dashSnaps` _result_2 _asgame_info_instance))))))

(fn `addDeath`
  (params (Character :type "/Game/Blueprints/enums/Character_Enums Enum" :default "NewEnumerator0"))
  (bind _asgame_info_instance (cast `/Game/Blueprints/Instance/gameInfo_instance` (`self.gameInfo_ref`)))
  (if (`|EnumEquality` Character "NewEnumerator0")
    (bind _result (`/Engine/EditorBlueprintResources/StandardMacros.IncrementInt` (`/Game/Blueprints/Instance/gameInfo_instance.Player_deaths` _asgame_info_instance))
      (:`  `
        (set `/Game/Blueprints/Instance/gameInfo_instance.Player_deaths` _result _asgame_info_instance)))
    (else
      (bind _result_2 (`/Engine/EditorBlueprintResources/StandardMacros.IncrementInt` (`/Game/Blueprints/Instance/gameInfo_instance.Enemy_deaths` _asgame_info_instance))
        (:`  `
          (set `/Game/Blueprints/Instance/gameInfo_instance.Enemy_deaths` _result_2 _asgame_info_instance))))))

(fn `addFightStarted`
  (bind _asgame_info_instance (cast `/Game/Blueprints/Instance/gameInfo_instance` (`self.gameInfo_ref`)))
  (bind _result (`/Engine/EditorBlueprintResources/StandardMacros.IncrementInt` (`/Game/Blueprints/Instance/gameInfo_instance.fightsStarted` _asgame_info_instance))
    (:`  `
      (set `/Game/Blueprints/Instance/gameInfo_instance.fightsStarted` _result _asgame_info_instance))))

(fn `addHealthHealed`
  (params (HealthHealed :type Integer) (Character :type "/Game/Blueprints/enums/Character_Enums Enum" :default "NewEnumerator0"))
  (bind _asgame_info_instance (cast `/Game/Blueprints/Instance/gameInfo_instance` (`self.gameInfo_ref`)))
  (if (`|EnumEquality` Character "NewEnumerator0")
    (set `/Game/Blueprints/Instance/gameInfo_instance.Player_healthHealed` (+ (`/Game/Blueprints/Instance/gameInfo_instance.Player_healthHealed` _asgame_info_instance) HealthHealed) _asgame_info_instance)
    (else
      (set `/Game/Blueprints/Instance/gameInfo_instance.Enemy_healthHealed` (+ (`/Game/Blueprints/Instance/gameInfo_instance.Enemy_healthHealed` _asgame_info_instance) HealthHealed) _asgame_info_instance))))

(fn `addHeavyBlock`
  (params (Character :type "/Game/Blueprints/enums/Character_Enums Enum" :default "NewEnumerator0"))
  (bind _asgame_info_instance (cast `/Game/Blueprints/Instance/gameInfo_instance` (`self.gameInfo_ref`)))
  (if (`|EnumEquality` Character "NewEnumerator0")
    (bind _result (`/Engine/EditorBlueprintResources/StandardMacros.IncrementInt` (`/Game/Blueprints/Instance/gameInfo_instance.Player_heavyBlocked` _asgame_info_instance))
      (:`  `
        (set `/Game/Blueprints/Instance/gameInfo_instance.Player_heavyBlocked` _result _asgame_info_instance)))
    (else
      (bind _result_2 (`/Engine/EditorBlueprintResources/StandardMacros.IncrementInt` (`/Game/Blueprints/Instance/gameInfo_instance.Enemy_heavyBlocked` _asgame_info_instance))
        (:`  `
          (set `/Game/Blueprints/Instance/gameInfo_instance.Enemy_heavyBlocked` _result_2 _asgame_info_instance))))))

(fn `addHeavyComboCompleted`
  (params (Character :type "/Game/Blueprints/enums/Character_Enums Enum" :default "NewEnumerator0"))
  (bind _asgame_info_instance (cast `/Game/Blueprints/Instance/gameInfo_instance` (`self.gameInfo_ref`)))
  (if (`|EnumEquality` Character "NewEnumerator0")
    (bind _result (`/Engine/EditorBlueprintResources/StandardMacros.IncrementInt` (`/Game/Blueprints/Instance/gameInfo_instance.Player_heavyComboCompleted` _asgame_info_instance))
      (:`  `
        (set `/Game/Blueprints/Instance/gameInfo_instance.Player_heavyComboCompleted` _result _asgame_info_instance)))
    (else
      (bind _result_2 (`/Engine/EditorBlueprintResources/StandardMacros.IncrementInt` (`/Game/Blueprints/Instance/gameInfo_instance.Enemy_heavyComboComplete` _asgame_info_instance))
        (:`  `
          (set `/Game/Blueprints/Instance/gameInfo_instance.Enemy_heavyComboComplete` _result_2 _asgame_info_instance))))))

(fn `addHeavyHit`
  (params (Character :type "/Game/Blueprints/enums/Character_Enums Enum" :default "NewEnumerator0"))
  (bind _asgame_info_instance (cast `/Game/Blueprints/Instance/gameInfo_instance` (`self.gameInfo_ref`)))
  (if (`|EnumEquality` Character "NewEnumerator0")
    (bind _result (`/Engine/EditorBlueprintResources/StandardMacros.IncrementInt` (`/Game/Blueprints/Instance/gameInfo_instance.Player_heavyHit` _asgame_info_instance))
      (:`  `
        (set `/Game/Blueprints/Instance/gameInfo_instance.Player_heavyHit` _result _asgame_info_instance)))
    (else
      (bind _result_2 (`/Engine/EditorBlueprintResources/StandardMacros.IncrementInt` (`/Game/Blueprints/Instance/gameInfo_instance.Enemy_heavyHit` _asgame_info_instance))
        (:`  `
          (set `/Game/Blueprints/Instance/gameInfo_instance.Enemy_heavyHit` _result_2 _asgame_info_instance))))))

(fn `addHeavySwing`
  (params (Character :type "/Game/Blueprints/enums/Character_Enums Enum" :default "NewEnumerator0"))
  (bind _asgame_info_instance (cast `/Game/Blueprints/Instance/gameInfo_instance` (`self.gameInfo_ref`)))
  (if (`|EnumEquality` Character "NewEnumerator0")
    (bind _result (`/Engine/EditorBlueprintResources/StandardMacros.IncrementInt` (`/Game/Blueprints/Instance/gameInfo_instance.Player_heavySwing` _asgame_info_instance))
      (:`  `
        (set `/Game/Blueprints/Instance/gameInfo_instance.Player_heavySwing` _result _asgame_info_instance)))
    (else
      (bind _result_2 (`/Engine/EditorBlueprintResources/StandardMacros.IncrementInt` (`/Game/Blueprints/Instance/gameInfo_instance.Enemy_heavySwing` _asgame_info_instance))
        (:`  `
          (set `/Game/Blueprints/Instance/gameInfo_instance.Enemy_heavySwing` _result_2 _asgame_info_instance))))))

(fn `addLightBlock`
  (params (Character :type "/Game/Blueprints/enums/Character_Enums Enum" :default "NewEnumerator0"))
  (bind _asgame_info_instance (cast `/Game/Blueprints/Instance/gameInfo_instance` (`self.gameInfo_ref`)))
  (if (`|EnumEquality` Character "NewEnumerator0")
    (bind _result (`/Engine/EditorBlueprintResources/StandardMacros.IncrementInt` (`/Game/Blueprints/Instance/gameInfo_instance.Player_lightBlocked` _asgame_info_instance))
      (:`  `
        (set `/Game/Blueprints/Instance/gameInfo_instance.Player_lightBlocked` _result _asgame_info_instance)))
    (else
      (bind _result_2 (`/Engine/EditorBlueprintResources/StandardMacros.IncrementInt` (`/Game/Blueprints/Instance/gameInfo_instance.Enemy_lightBlocked` _asgame_info_instance))
        (:`  `
          (set `/Game/Blueprints/Instance/gameInfo_instance.Enemy_lightBlocked` _result_2 _asgame_info_instance))))))

(fn `addLightComboCompleted`
  (params (Character :type "/Game/Blueprints/enums/Character_Enums Enum" :default "NewEnumerator0"))
  (bind _asgame_info_instance (cast `/Game/Blueprints/Instance/gameInfo_instance` (`self.gameInfo_ref`)))
  (if (`|EnumEquality` Character "NewEnumerator0")
    (bind _result (`/Engine/EditorBlueprintResources/StandardMacros.IncrementInt` (`/Game/Blueprints/Instance/gameInfo_instance.Player_lightComboComplete` _asgame_info_instance))
      (:`  `
        (set `/Game/Blueprints/Instance/gameInfo_instance.Player_lightComboComplete` _result _asgame_info_instance)))
    (else
      (bind _result_2 (`/Engine/EditorBlueprintResources/StandardMacros.IncrementInt` (`/Game/Blueprints/Instance/gameInfo_instance.Enemy_lightComboComplete` _asgame_info_instance))
        (:`  `
          (set `/Game/Blueprints/Instance/gameInfo_instance.Enemy_lightComboComplete` _result_2 _asgame_info_instance))))))

(fn `addLightHit`
  (params (Character :type "/Game/Blueprints/enums/Character_Enums Enum" :default "NewEnumerator0"))
  (bind _asgame_info_instance (cast `/Game/Blueprints/Instance/gameInfo_instance` (`self.gameInfo_ref`)))
  (if (`|EnumEquality` Character "NewEnumerator0")
    (bind _result (`/Engine/EditorBlueprintResources/StandardMacros.IncrementInt` (`/Game/Blueprints/Instance/gameInfo_instance.Player_lightHit` _asgame_info_instance))
      (:`  `
        (set `/Game/Blueprints/Instance/gameInfo_instance.Player_lightHit` _result _asgame_info_instance)))
    (else
      (bind _result_2 (`/Engine/EditorBlueprintResources/StandardMacros.IncrementInt` (`/Game/Blueprints/Instance/gameInfo_instance.Enemy_lightHit` _asgame_info_instance))
        (:`  `
          (set `/Game/Blueprints/Instance/gameInfo_instance.Enemy_lightHit` _result_2 _asgame_info_instance))))))

(fn `addLightSwing`
  (params (Character :type "/Game/Blueprints/enums/Character_Enums Enum" :default "NewEnumerator0"))
  (bind _asgame_info_instance (cast `/Game/Blueprints/Instance/gameInfo_instance` (`self.gameInfo_ref`)))
  (if (`|EnumEquality` Character "NewEnumerator0")
    (bind _result (`/Engine/EditorBlueprintResources/StandardMacros.IncrementInt` (`/Game/Blueprints/Instance/gameInfo_instance.Player_lightSwing` _asgame_info_instance))
      (:`  `
        (set `/Game/Blueprints/Instance/gameInfo_instance.Player_lightSwing` _result _asgame_info_instance)))
    (else
      (`/Engine/EditorBlueprintResources/StandardMacros.IncrementInt` (`/Game/Blueprints/Instance/gameInfo_instance.Enemy_lightSwing` _asgame_info_instance)
        (:`  `
          (set `/Game/Blueprints/Instance/gameInfo_instance.Enemy_lightSwing` 0 _asgame_info_instance))))))

(fn `addProjectileFired`
  (params (Character :type "/Game/Blueprints/enums/Character_Enums Enum" :default "NewEnumerator0"))
  (`KismetSystemLibrary.PrintString` "projectile: fix when finished"))

(fn `addProjectileHit`
  (`KismetSystemLibrary.PrintString` "projectile: fix when finished"))

(fn `addTimeSpentFloating`
  (params (TimeSpentFloating :type "Float (double-precision)") (Character :type "/Game/Blueprints/enums/Character_Enums Enum" :default "NewEnumerator0"))
  (bind _asgame_info_instance (cast `/Game/Blueprints/Instance/gameInfo_instance` (`self.gameInfo_ref`)))
  (if (`|EnumEquality` Character "NewEnumerator0")
    (set `/Game/Blueprints/Instance/gameInfo_instance.Player_timeSpentFloating` (+ (`/Game/Blueprints/Instance/gameInfo_instance.Player_timeSpentFloating` _asgame_info_instance) TimeSpentFloating) _asgame_info_instance)
    (else
      (set `/Game/Blueprints/Instance/gameInfo_instance.Enemy_timeSpentFloating` (+ (`/Game/Blueprints/Instance/gameInfo_instance.Enemy_timeSpentFloating` _asgame_info_instance) TimeSpentFloating) _asgame_info_instance))))

(fn `calculateTimeSpentFloating`
  (params (`Delta Seconds` :type "Float (double-precision)"))
  (bind _player_floattimer (`self.Player_floatTimer`))
  (bind _enemy_floattimer (`self.Enemy_floatTimer`))
  (`|ExecutionSequence`
    (:`then_0`
      (if (== (`CharacterMovementComponent.GravityScale` (`Character.CharacterMovement` (`self.playerRef`))) 0.0)
        (set `self.Player_floatTimer` (+ _player_floattimer `Delta Seconds`))
        (else
          (`self.addTimeSpentFloating` _player_floattimer "NewEnumerator0")
          (set `self.Player_floatTimer` 0.0))))
    (:`then_1`
      (if (== (`CharacterMovementComponent.GravityScale` (`Character.CharacterMovement` (`self.enemyRef`))) 0.0)
        (set `self.Enemy_floatTimer` (+ _enemy_floattimer `Delta Seconds`))
        (else
          (`self.addTimeSpentFloating` _enemy_floattimer "NewEnumerator1")
          (set `self.Enemy_floatTimer` 0.0))))))

(fn `UserConstructionScript`)