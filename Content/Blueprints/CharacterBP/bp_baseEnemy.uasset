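; Base enemy Blueprint that publishes its world location as the boss location.
; BeginPlay starts a looping timer that calls location_send five times a second, avoiding Tick.
; That function casts the Game Instance to gameInfo_instance and writes the actor's location into BossLocation, with debug prints on success or failure.
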(event `self.ReceiveBeginPlay`
  (`parent.ReceiveBeginPlay`)
  (`KismetSystemLibrary.K2_SetTimer` null "location_send" 0.2 true))

(fn `location_send`
  (bind _asgame_info_instance (cast `/Game/Blueprints/Instance/gameInfo_instance` (`GameplayStatics.GetGameInstance`))
    (:`then`
      (set `/Game/Blueprints/Instance/gameInfo_instance.bossLocation` (`self.K2_GetActorLocation`) _asgame_info_instance)
      (`KismetSystemLibrary.PrintString` "Hello"))
    (:`CastFailed`
      (`KismetSystemLibrary.PrintString` "ohNo"))))

(fn `UserConstructionScript`
  (`parent.UserConstructionScript`))