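; Base player character with camera-relative movement, jump with one air jump, four-way dash and boss lock-on.
; A per-tick ground trace drives air state; inputs play montages, while separate functions apply launches, with dash re-launching on a timer.
; Lock-on turns camera and actor toward the GameInstance's boss location, tightening pitch up close, but its update timeline is unwired.
; Action gating, buffer consumption and several helpers are empty stubs.
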(event `self.ReceiveTick`
  (params (DeltaSeconds :type "Float (single-precision)"))
  (`self.ground_check`))

(event `self.ReceiveBeginPlay`
  (set `self.animInst_mesh` (`SkeletalMeshComponent.GetAnimInstance` (`self.Mesh`)))
  (`self.check_getEnemy`))

(event `InputAxis|Turn` :overrideparent false
  (params (AxisValue :type "Float (single-precision)"))
  ;[0.4792 0 0.02079] inputs
  ;;[1 1 1] Carmera
  ;;;[1 1 1] mouseInput
  (`self.AddControllerYawInput` AxisValue))

(event `InputAction|Jump`
  (params (Key :type "Key Structure"))
  (:`Pressed`
    (`self.jump_logic`)))

(event `InputAxis|LookUp` :overrideparent false
  (params (AxisValue :type "Float (single-precision)"))
  ;[0.4792 0 0.02079] inputs
  ;;[1 1 1] Carmera
  ;;;[1 1 1] mouseInput
  (`self.AddControllerPitchInput` AxisValue))

(event `InputAction|Dash`
  (params (Key :type "Key Structure"))
  (:`Pressed`
    (`self.dash_logic`)))

(event `InputAction|LockOn`
  (params (Key :type "Key Structure"))
  (:`Pressed`
    (`self.lockOn_logic`)))

(event `InputAxis|TurnRate`
  (params (AxisValue :type "Float (single-precision)"))
  ;[0.4792 0 0.02079] inputs
  ;;[1 1 1] Carmera
  ;;;[1 1 1] Controller Input
  (`self.AddControllerYawInput` (* AxisValue (`self.BaseTurnRate`) (`GameplayStatics.GetWorldDeltaSeconds`))))

(event `InputAxis|LookUpRate`
  (params (AxisValue :type "Float (single-precision)"))
  ;[0.4792 0 0.02079] inputs
  ;;[1 1 1] Carmera
  ;;;[1 1 1] Controller Input
  (`self.AddControllerPitchInput` (* AxisValue (`self.BaseLookUpRate`) (`GameplayStatics.GetWorldDeltaSeconds`))))

(event `InputAxis|MoveForward`
  (params (AxisValue :type "Float (single-precision)"))
  ;[0.4792 0 0.02079] inputs
  ;;[1 1 1] Movement
  (if true
    (`self.AddMovementInput` (`KismetMathLibrary.GetForwardVector` (`KismetMathLibrary.MakeRotator` 0.0 0.0 (.yaw (`self.GetControlRotation`)))) AxisValue)))

(event `InputAxis|MoveRight`
  (params (AxisValue :type "Float (single-precision)"))
  ;[0.4792 0 0.02079] inputs
  ;;[1 1 1] Movement
  (if true
    (`self.AddMovementInput` (`KismetMathLibrary.GetRightVector` (`KismetMathLibrary.MakeRotator` 0.0 0.0 (.yaw (`self.GetControlRotation`)))) AxisValue)))

(event `LockOn_TimelineStart`
  (`/Engine/EditorBlueprintResources/StandardMacros.Gate` true :!via `Toggle`
    (:`Exit`
      (`self.lockOn_update`))))

(fn `AI_canAct`
  (params (Yes :type Boolean :default true)))

(fn `buffer_canUse?`
  (returns (`?` :type Boolean))
  (if (`self.buffer_selected`)
    _
    (elif (`self.buffer_canInput?`)
      (return true)
      (else
        _)))
  (return false))

(fn `buffer_input`
  (params (NewParam :type "/Game/Blueprints/enums/enum_BufferInputs Enum" :default "NewEnumerator2"))
  (set `self.buffer_selected` true)
  (set `self.buffer_Action` NewParam))

(fn `buffer_logic`)

(fn `call_Montage`
  (params (PlayerAnimation :type "AnimMontage Object Reference") (PlayRate :type "Float (double-precision)" :default 1.0) (StopActiveMontage :type Boolean :default true))
  (returns (Duration :type "Float (double-precision)"))
  (bind _returnvalue (`AnimInstance.Montage_Play` (`self.animInst_mesh`) PlayerAnimation PlayRate "Duration" 0.0 StopActiveMontage))
  (return _returnvalue))

(fn `cameraFOV_set`
  (params (`FOV subtraction` :type "Float (double-precision)"))
  (bind _maincamera (`self.mainCamera`))
  (`CameraComponent.SetFieldOfView` _maincamera (- (`CameraComponent.FieldOfView` _maincamera) `FOV subtraction`)))

(fn `check_getEnemy`
  (bind _outactors (`GameplayStatics.GetAllActorsOfClass` "bp_baseChar_C"))
  (for _array_element _outactors
    (if (not (== _array_element self))
      (set `self.Enemy` _array_element))))

(fn `check_outline`
  (params (On :type Boolean))
  (bind _mesh (`self.Mesh`))
  (if On
    (`PrimitiveComponent.SetRenderCustomDepth` _mesh true)
    (else
      (`PrimitiveComponent.SetRenderCustomDepth` _mesh false))))

(fn `dash_active`
  (if (`|EnumEquality` (`self.state_current`) "NewEnumerator6")
    (`self.LaunchCharacter` (`self.Dash_Direction`) true true)
    (`self.cameraFOV_set` -0.3)
    (`KismetSystemLibrary.K2_SetTimer` null "dash_active" 0.01)))

(fn `dash_B`
  (set `self.state_dashInput` "NewEnumerator1")
  (`self.call_Montage` (`|GetArrayItem` (`self.animations_dash`) 1) (`self.AnimationRate_Dash`)))

(fn `dash_F`
  (set `self.state_dashInput` "NewEnumerator0")
  (`self.call_Montage` (`|GetArrayItem` (`self.animations_dash`)) (`self.AnimationRate_Dash`)))

(fn `dash_inputCheck`
  (returns (InputDirection :type "/Game/Blueprints/enums/Input_Enums Enum"))
  (if (>= (`self.GetInputAxisValue`) 0.5)
    (return "NewEnumerator0")
    (elif (<= (`self.GetInputAxisValue`) -0.5)
      (return "NewEnumerator1")
      (elif (<= (`self.GetInputAxisValue`) -0.5)
        (return "NewEnumerator2")
        (elif (>= (`self.GetInputAxisValue`) 0.5)
          (return "NewEnumerator3")
          (else
            (return "NewEnumerator0")))))))

(fn `dash_L`
  (set `self.state_dashInput` "NewEnumerator2")
  (`self.call_Montage` (`|GetArrayItem` (`self.animations_dash`) 2) (`self.AnimationRate_Dash`)))

(fn `dash_logic`
  (if (`self.canUseAction?`)
    (set `self.state_current` "NewEnumerator6")
    (set `self.state_inIdle?` false)
    (`self.slowMotionReset`)
    (bind _inputdirection (`self.dash_inputCheck`))
    (switch `/Game/Blueprints/enums/Input_Enums` _inputdirection
      (:`NewEnumerator0`
        (if (not (`self.state_targetLocked`))
          (`self.dash_F`)))
      (:`NewEnumerator1`
        (if (not (`self.state_targetLocked`))
          (`self.dash_B`)))
      (:`NewEnumerator2`
        (`self.dash_L`))
      (:`NewEnumerator3`
        (`self.dash_R`)))
    (else
      (bind __ (`self.buffer_canUse?`))
      (if __
        (`self.buffer_input` "NewEnumerator4")))))

(fn `dash_R`
  (set `self.state_dashInput` "NewEnumerator3")
  (`self.call_Montage` (`|GetArrayItem` (`self.animations_dash`) 3) (`self.AnimationRate_Dash`)))

(fn `dash_reset`
  (bind _charactermovement (`self.CharacterMovement`))
  (set `self.state_current` "NewEnumerator0")
  (set `self.state_inIdle?` true)
  (`CameraComponent.SetFieldOfView` (`self.mainCamera`) 90.0)
  (set `CharacterMovementComponent.GroundFriction` 8.0 _charactermovement)
  (set `CharacterMovementComponent.FallingLateralFriction` 10.0 _charactermovement)
  (`KismetSystemLibrary.K2_SetTimer` null "lateralFriction_Off" 0.1)
  (`self.buffer_logic`)
  (`self.AI_canAct` true))

(fn `dash_Snap`)

(fn `dash_start`
  (switch `/Game/Blueprints/enums/Input_Enums` (`self.state_dashInput`)
    (:`NewEnumerator0`
      (set `self.Dash_Direction` (* (`self.GetActorForwardVector`) (`self.dash_rate`))))
    (:`NewEnumerator1`
      (set `self.Dash_Direction` (* (`self.GetActorForwardVector`) (* (`self.dash_rate`) -1.0))))
    (:`NewEnumerator2`
      (set `self.Dash_Direction` (* (`self.GetActorRightVector`) (* (`self.dash_rate`) -1.0))))
    (:`NewEnumerator3`
      (set `self.Dash_Direction` (* (`self.GetActorRightVector`) (`self.dash_rate`)))))
  (`self.dash_active`))

(fn `ground_check`
  (bind _returnvalue (`self.K2_GetActorLocation`))
  (bind (_outhits _returnvalue_2) (`KismetSystemLibrary.LineTraceMulti` _returnvalue (`KismetMathLibrary.MakeVector` (.x _returnvalue) (.y _returnvalue) (- (.z _returnvalue) 200.0)) "TraceTypeQuery3"))
  (if _returnvalue_2
    (if (`self.state_inAir?`)
      (`self.call_Montage` (`|GetArrayItem` (`self.animations_movement`) 1) 1.0 false)
      (set `self.state_inAir?` false)
      (set `self.state_hasJumped?` false))
    (else
      (set `self.state_inAir?` true))))

(fn `jump_action`
  (`self.LaunchCharacter` (* (0.0 0.0 1.0) 3500.0) false true)
  (`self.jump_spawnParticle`))

(fn `jump_logic`
  (if (`self.state_inAir?`)
    (if (`self.state_hasJumped?`)
      _
      (elif (`self.canUseAction?`)
        (set `self.state_hasJumped?` true)
        (`self.call_Montage` (`|GetArrayItem` (`self.animations_movement`)) :!label _label)))
    (elif (`self.canUseAction?`)
      (goto _label))))

(fn `jump_spawnParticle`
  (`GameplayStatics.SpawnEmitterAtLocation` (`self.jump_particle`) (`KismetMathLibrary.MakeVector` (.x (`SceneComponent.K2_GetComponentLocation` (`self.Mesh`))) (.y (`SceneComponent.K2_GetComponentLocation` (`self.Mesh`))) (+ (.z (`SceneComponent.K2_GetComponentLocation` (`self.Mesh`))) 100.0)) (struct) (`self.jump_particleSize`)))

(fn `lateralFriction_Off`)

(fn `lateralFriction_On`)

(fn `lockOn_logic`
  (bind _charactermovement (`self.CharacterMovement`))
  (bind _enemy (`self.Enemy`))
  (`/Engine/EditorBlueprintResources/StandardMacros.IsValid` (`self.Enemy`)
    (:`Is Valid`
      (if (`self.state_targetLocked`)
        (set `self.state_targetLocked` false)
        (set `CharacterMovementComponent.bOrientRotationToMovement` true _charactermovement)
        (`self.check_outline` _enemy false)
        (else
          (set `self.state_targetLocked` true)
          (set `CharacterMovementComponent.bOrientRotationToMovement` false _charactermovement)
          (if (`self.state_dashSnapInRange`)
            (`self.check_outline` _enemy true))))
      (bind _outactors (`GameplayStatics.GetAllActorsOfClass` "/Game/Blueprints/CharacterBP/bp_baseEnemy.bp_baseEnemy_C"))
      (message `/Game/Blueprints/Interface/EnemyInteraction.LockOn` _outactors)
      (`self.LockOn_TimelineStart`))))

(fn `lockOn_update`
  (bind _returnvalue (`KismetMathLibrary.VSize` (- (`self.K2_GetActorLocation`) (`self.K2_GetActorLocation` (`self.Enemy`)))))
  (bind _returnvalue_2 (/ _returnvalue 400.0))
  ;[1 1 1] check enemy is valid
  (`/Engine/EditorBlueprintResources/StandardMacros.IsValid` (`self.Enemy`)
    (:`Is Valid`
      (bind _asgame_info_instance (cast `/Game/Blueprints/Instance/gameInfo_instance` (`GameplayStatics.GetGameInstance`)))
      ;[1 1 1] check distance
      (if (> _returnvalue 400.0)
        ;[1 1 1] default lock on logic
        (if (and (not (`self.state_onCieling`)) (not (`self.state_onWall?`)))
          (bind _bosslocation (`/Game/Blueprints/Instance/gameInfo_instance.bossLocation` _asgame_info_instance))
          (bind _yaw (.yaw (`KismetMathLibrary.RInterpTo` (`KismetMathLibrary.MakeRotator` (.roll (`Controller.GetControlRotation` (`self.GetController`))) (.pitch (`Controller.GetControlRotation` (`self.GetController`))) (.yaw (`Controller.GetControlRotation` (`self.GetController`)))) (`KismetMathLibrary.MakeRotator` (.roll (`KismetMathLibrary.FindLookAtRotation` (`SceneComponent.K2_GetComponentLocation` (`self.Mesh`)) _bosslocation)) (.pitch (`KismetMathLibrary.FindLookAtRotation` (`SceneComponent.K2_GetComponentLocation` (`self.Mesh`)) _bosslocation)) (.yaw (`KismetMathLibrary.FindLookAtRotation` (`SceneComponent.K2_GetComponentLocation` (`self.Mesh`)) _bosslocation))) (`GameplayStatics.GetWorldDeltaSeconds`) 25.0)))
          (bind _returnvalue_3 (`KismetMathLibrary.MakeRotator` (.roll (`KismetMathLibrary.RInterpTo` (`KismetMathLibrary.MakeRotator` (.roll (`Controller.GetControlRotation` (`self.GetController`))) (.pitch (`Controller.GetControlRotation` (`self.GetController`))) (.yaw (`Controller.GetControlRotation` (`self.GetController`)))) (`KismetMathLibrary.MakeRotator` (.roll (`KismetMathLibrary.FindLookAtRotation` (`SceneComponent.K2_GetComponentLocation` (`self.Mesh`)) _bosslocation)) (.pitch (`KismetMathLibrary.FindLookAtRotation` (`SceneComponent.K2_GetComponentLocation` (`self.Mesh`)) _bosslocation)) (.yaw (`KismetMathLibrary.FindLookAtRotation` (`SceneComponent.K2_GetComponentLocation` (`self.Mesh`)) _bosslocation))) (`GameplayStatics.GetWorldDeltaSeconds`) 25.0)) (`KismetMathLibrary.FClamp` (.pitch (`KismetMathLibrary.RInterpTo` (`KismetMathLibrary.MakeRotator` (.roll (`Controller.GetControlRotation` (`self.GetController`))) (.pitch (`Controller.GetControlRotation` (`self.GetController`))) (.yaw (`Controller.GetControlRotation` (`self.GetController`)))) (`KismetMathLibrary.MakeRotator` (.roll (`KismetMathLibrary.FindLookAtRotation` (`SceneComponent.K2_GetComponentLocation` (`self.Mesh`)) _bosslocation)) (.pitch (`KismetMathLibrary.FindLookAtRotation` (`SceneComponent.K2_GetComponentLocation` (`self.Mesh`)) _bosslocation)) (.yaw (`KismetMathLibrary.FindLookAtRotation` (`SceneComponent.K2_GetComponentLocation` (`self.Mesh`)) _bosslocation))) (`GameplayStatics.GetWorldDeltaSeconds`) 25.0)) -180.0 60.0) _yaw))
          (`Controller.SetControlRotation` (`self.GetController`) _returnvalue_3)
          (bind _returnvalue_4 (`KismetMathLibrary.MakeRotator` 0.0 0.0 _yaw))
          (`self.K2_SetActorRotation` _returnvalue_4))
        (else
          ;[1 1 1] lock on logic if player is to close
          (if (and (not (`self.state_onCieling`)) (not (`self.state_onWall?`)))
            (bind _yaw_2 (.yaw (`KismetMathLibrary.RInterpTo` (`KismetMathLibrary.MakeRotator` (.roll (`Controller.GetControlRotation` (`self.GetController`))) (.pitch (`Controller.GetControlRotation` (`self.GetController`))) (.yaw (`Controller.GetControlRotation` (`self.GetController`)))) (`KismetMathLibrary.MakeRotator` (.roll (`KismetMathLibrary.FindLookAtRotation` (`SceneComponent.K2_GetComponentLocation` (`self.Mesh`)) _bosslocation)) (.pitch (`KismetMathLibrary.FindLookAtRotation` (`SceneComponent.K2_GetComponentLocation` (`self.Mesh`)) _bosslocation)) (.yaw (`KismetMathLibrary.FindLookAtRotation` (`SceneComponent.K2_GetComponentLocation` (`self.Mesh`)) _bosslocation))) (`GameplayStatics.GetWorldDeltaSeconds`) 25.0)))
            (`Controller.SetControlRotation` (`self.GetController`) (`KismetMathLibrary.RLerp` (`KismetMathLibrary.MakeRotator` (.roll (`KismetMathLibrary.RInterpTo` (`KismetMathLibrary.MakeRotator` (.roll (`Controller.GetControlRotation` (`self.GetController`))) (.pitch (`Controller.GetControlRotation` (`self.GetController`))) (.yaw (`Controller.GetControlRotation` (`self.GetController`)))) (`KismetMathLibrary.MakeRotator` (.roll (`KismetMathLibrary.FindLookAtRotation` (`SceneComponent.K2_GetComponentLocation` (`self.Mesh`)) _bosslocation)) (.pitch (`KismetMathLibrary.FindLookAtRotation` (`SceneComponent.K2_GetComponentLocation` (`self.Mesh`)) _bosslocation)) (.yaw (`KismetMathLibrary.FindLookAtRotation` (`SceneComponent.K2_GetComponentLocation` (`self.Mesh`)) _bosslocation))) (`GameplayStatics.GetWorldDeltaSeconds`) 25.0)) (`KismetMathLibrary.FClamp` (.pitch (`KismetMathLibrary.RInterpTo` (`KismetMathLibrary.MakeRotator` (.roll (`Controller.GetControlRotation` (`self.GetController`))) (.pitch (`Controller.GetControlRotation` (`self.GetController`))) (.yaw (`Controller.GetControlRotation` (`self.GetController`)))) (`KismetMathLibrary.MakeRotator` (.roll (`KismetMathLibrary.FindLookAtRotation` (`SceneComponent.K2_GetComponentLocation` (`self.Mesh`)) _bosslocation)) (.pitch (`KismetMathLibrary.FindLookAtRotation` (`SceneComponent.K2_GetComponentLocation` (`self.Mesh`)) _bosslocation)) (.yaw (`KismetMathLibrary.FindLookAtRotation` (`SceneComponent.K2_GetComponentLocation` (`self.Mesh`)) _bosslocation))) (`GameplayStatics.GetWorldDeltaSeconds`) 25.0)) -180.0 0.0) _yaw_2) _returnvalue_3 _returnvalue_2 true))
            (`self.K2_SetActorRotation` (`KismetMathLibrary.RLerp` (`KismetMathLibrary.MakeRotator` 0.0 0.0 _yaw_2) _returnvalue_4 _returnvalue_2 true))))))
    (:`Is Not Valid`
      (`self.lockOn_logic`))))

(fn `slowMotionReset`
  (if (`self.state_inSlowMo`)
    (set `self.state_inSlowMo` false)
    (`GameplayStatics.SetGlobalTimeDilation` 1.0)))

(fn `UserConstructionScript`)