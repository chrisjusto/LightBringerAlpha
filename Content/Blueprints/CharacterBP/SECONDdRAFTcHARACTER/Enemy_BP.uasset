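; Enemy boss Blueprint that reports its position and fires volleys of projectiles.
; After a short BeginPlay delay, unless player-controlled, it runs a fast looping timer that writes its location to BossLocation in the game instance.
; SpawnProjectile spawns projectiles at five arrow components and stores them; ShootProjectile launches every stored one along its forward vector, never clearing the array.
; The Lockon event alternately shows and hides the lock-on UI.
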(event `self.ReceiveBeginPlay`
  (`parent.ReceiveBeginPlay`)
  (`KismetSystemLibrary.Delay` 1.0)
  (if (not (== self (`Controller.K2_GetPawn` (`GameplayStatics.GetPlayerController` 0))))
    (`KismetSystemLibrary.K2_SetTimer` null "sendLocation" 0.005 true)))

(event `self.ReceiveTick`
  (params (DeltaSeconds :type "Float (single-precision)"))
  (`parent.ReceiveTick` DeltaSeconds))

(event `/Game/Blueprints/Interface/EnemyInteraction.LockOn`
  (`/Engine/EditorBlueprintResources/StandardMacros.FlipFlop`
    (:`A`
      (`SceneComponent.SetHiddenInGame` (`self.LockOnUI`) false false))
    (:`B`
      (`SceneComponent.SetHiddenInGame` (`self.LockOnUI`) true false))))

(event `self.shootProjectile`
  (for (_array_element _array_index) (`self.ENEMYProjectile`)
    (`/Game/Blueprints/Projectiles/BP_playerProjectile.LaunchatEnemy` _array_element (`SceneComponent.GetForwardVector` (`/Game/Blueprints/Projectiles/BP_playerProjectile.DefaultSceneRoot` _array_element)) null null)))

(event `self.spawnProjectile`
  (for _array_element (`self.Arrows`)
    (bind _returnvalue (`|SpawnActorFromClass` "/Game/Blueprints/Projectiles/BP_enemyProjectile.BP_enemyProjectile_C" (`SceneComponent.K2_GetComponentToWorld` _array_element) "Undefined" "OverrideRootScale" null null))
    (`KismetArrayLibrary.Array_Add` (`self.ENEMYProjectile`) _returnvalue)))

(fn `sendLocation`
  (bind _asgame_info_instance (cast `/Game/Blueprints/Instance/gameInfo_instance` (`GameplayStatics.GetGameInstance`)))
  (set `/Game/Blueprints/Instance/gameInfo_instance.bossLocation` (`self.K2_GetActorLocation`) _asgame_info_instance))

(fn `UserConstructionScript`
  (`parent.UserConstructionScript`)
  (set `self.Arrows` (`|MakeArray` (`self.Arrow5`) (`self.Arrow4`) (`self.Arrow3`) (`self.Arrow2`) (`self.Arrow1`))))