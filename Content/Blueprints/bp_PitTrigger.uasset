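; Pit trigger volume that tracks a player and an enemy bp_baseCharacter inside it, told apart by their Character enum.
; A looping one-second timer checks occupancy, setting a flag when both are present or starting recovery for a lone occupant.
; Enemy recovery marks it stuck, waits, then launches it straight up and clears the state.
; Player recovery contains only a delay, and the both-present flag triggers nothing further here.
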(event `self.ReceiveBeginPlay`
  (`KismetSystemLibrary.K2_SetTimer` null "check_BothParties" 1.0 true))

(event `self.ReceiveActorBeginOverlap`
  (params (OtherActor :type "Actor Object Reference"))
  (bind _asbp_base_character (cast `/Game/Blueprints/CharacterBP/bp_baseCharacter` OtherActor))
  (if (`|EnumEquality` (`/Game/Blueprints/CharacterBP/bp_baseCharacter.character` _asbp_base_character) "NewEnumerator0")
    (set `self.Player` _asbp_base_character)
    (else
      (set `self.Enemy` _asbp_base_character))))

(event `self.CollisionComponent.OnComponentEndOverlap`
  (params (OverlappedComponent :type "PrimitiveComponent Object Reference") (OtherActor :type "Actor Object Reference") (OtherComp :type "PrimitiveComponent Object Reference") (OtherBodyIndex :type Integer))
  (bind _asbp_base_character (cast `/Game/Blueprints/CharacterBP/bp_baseCharacter` OtherActor))
  (if (`|EnumEquality` (`/Game/Blueprints/CharacterBP/bp_baseCharacter.character` _asbp_base_character) "NewEnumerator0")
    (set `self.Player` null)
    (else
      (set `self.Enemy` null))))

(event `player recovery`
  (`KismetSystemLibrary.Delay` 5.0))

(event `enemy recovery`
  (bind _enemy (`self.Enemy`))
  (set `/Game/Blueprints/CharacterBP/bp_baseCharacter.state_stuck` true _enemy)
  (`KismetSystemLibrary.Delay` 5.0)
  (`Character.LaunchCharacter` (`self.Enemy`) (0.0 0.0 5000.0) true true)
  (set `/Game/Blueprints/CharacterBP/bp_baseCharacter.state_stuck` false _enemy))

(fn `check_BothParties`
  (bind _returnvalue (`KismetSystemLibrary.IsValid` (`self.Enemy`)))
  (bind _returnvalue_2 (`KismetSystemLibrary.IsValid` (`self.Player`)))
  (if (and _returnvalue_2 _returnvalue)
    (set `self.botharevalid` true)
    (elif _returnvalue_2
      (`self.player recovery`)
      (elif _returnvalue
        (`self.enemy recovery`)))))

(fn `UserConstructionScript`)