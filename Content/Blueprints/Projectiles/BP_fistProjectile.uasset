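; Fist projectile actor that charges up a ball, then launches it at a locked-on enemy or straight ahead of the player.
; On BeginPlay a timeline grows the sphere to full scale while a short delay runs.
; It then calls LaunchatEnemy, aimed at the enemy if the player is target-locked, otherwise along the player's forward vector.
; Afterward it destroys the Fists component and only then calls parent BeginPlay.
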(event `self.ReceiveBeginPlay`
  (bind _player (`self.Player`))
  (bind _enemy (`self.Enemy`))
  (`self.BallCharge`)
  (`KismetSystemLibrary.Delay` 0.5)
  (if (`/Game/Blueprints/CharacterBP/bp_baseCharacter.targetLocked?` _player)
    (`self.LaunchatEnemy` (`KismetMathLibrary.GetForwardVector` (`KismetMathLibrary.FindLookAtRotation` (`self.K2_GetActorLocation` _player) (`self.K2_GetActorLocation` _enemy))) _player _enemy)
    (else
      (`self.LaunchatEnemy` (`self.GetActorForwardVector` _player) _player _enemy)))
  (`ActorComponent.K2_DestroyComponent` (`self.Fists`))
  (`parent.ReceiveBeginPlay`))

(event `BallCharge`
  (set `self.ballScale` (`SceneComponent.K2_GetComponentScale` (`self.Sphere`)))
  (bind (_direction _newtrack_0) (`Timeline|Ball` :!via `PlayFromStart`)
    (:`Update`
      (`SceneComponent.SetRelativeScale3D` (`self.Sphere`) (`KismetMathLibrary.VLerp` (`self.ballScale`) (1.0 1.0 1.0) _newtrack_0)))))

(fn `UserConstructionScript`
  (`parent.UserConstructionScript`))