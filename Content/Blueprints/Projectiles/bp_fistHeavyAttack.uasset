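; Short-lived heavy fist attack actor that damages what it hits and destroys itself after a brief delay.
; Four static-mesh arms feed DealDamage, which removes the arm and damages the stored Enemy, launching it and destroying the actor unless the hit counter reaches four.
; The skeletal mesh overlap instead applies damage and hitstun to Player, despite excluding Player as the overlapped actor.
; Logic firing the arms toward Enemy is unconnected.
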(event `self.ReceiveBeginPlay`
  (`KismetSystemLibrary.Delay` 1.5)
  (`self.K2_DestroyActor`))

(event `self.StaticMesh.OnComponentBeginOverlap`
  (params (OverlappedComponent :type "PrimitiveComponent Object Reference") (OtherActor :type "Actor Object Reference") (OtherComp :type "PrimitiveComponent Object Reference") (OtherBodyIndex :type Integer) (bFromSweep :type Boolean) (SweepResult :type "HitResult Structure (by ref)"))
  (`self.dealDamage` OtherActor (`self.StaticMesh`)))

(event `self.StaticMesh1.OnComponentBeginOverlap`
  (params (OverlappedComponent :type "PrimitiveComponent Object Reference") (OtherActor :type "Actor Object Reference") (OtherComp :type "PrimitiveComponent Object Reference") (OtherBodyIndex :type Integer) (bFromSweep :type Boolean) (SweepResult :type "HitResult Structure (by ref)"))
  (`self.dealDamage` OtherActor (`self.StaticMesh1`)))

(event `self.StaticMesh2.OnComponentBeginOverlap`
  (params (OverlappedComponent :type "PrimitiveComponent Object Reference") (OtherActor :type "Actor Object Reference") (OtherComp :type "PrimitiveComponent Object Reference") (OtherBodyIndex :type Integer) (bFromSweep :type Boolean) (SweepResult :type "HitResult Structure (by ref)"))
  (`self.dealDamage` OtherActor (`self.StaticMesh2`)))

(event `self.StaticMesh3.OnComponentBeginOverlap`
  (params (OverlappedComponent :type "PrimitiveComponent Object Reference") (OtherActor :type "Actor Object Reference") (OtherComp :type "PrimitiveComponent Object Reference") (OtherBodyIndex :type Integer) (bFromSweep :type Boolean) (SweepResult :type "HitResult Structure (by ref)"))
  (`self.dealDamage` OtherActor (`self.StaticMesh3`)))

(event `self.SkeletalMesh.OnComponentBeginOverlap`
  (params (OverlappedComponent :type "PrimitiveComponent Object Reference") (OtherActor :type "Actor Object Reference") (OtherComp :type "PrimitiveComponent Object Reference") (OtherBodyIndex :type Integer) (bFromSweep :type Boolean) (SweepResult :type "HitResult Structure (by ref)"))
  (bind _player (`self.player`))
  (if (!= OtherActor _player)
    (`PrimitiveComponent.SetCollisionEnabled` (`self.SkeletalMesh`) "NoCollision")
    (`/Game/Blueprints/CharacterBP/bp_baseCharacter.Damage_set` _player 150 2.0 (0.0 0.0 0.0) "NewEnumerator0" 3000.0)
    (`/Game/Blueprints/CharacterBP/bp_baseCharacter.Hitsun_Logic` _player)
    (`self.K2_DestroyActor`)))

(fn `dealDamage`
  (params (Actor :type "Actor Object Reference") (Arm :type "PrimitiveComponent Object Reference"))
  (bind _player (`self.player`))
  (bind _enemy (`self.enemy`))
  (if (!= Actor _player)
    (`KismetSystemLibrary.PrintString` "Hello")
    (`PrimitiveComponent.SetCollisionEnabled` Arm "NoCollision")
    (`ActorComponent.K2_DestroyComponent` Arm)
    (bind _output_get (set `self.hit counter` (+ (`self.hit counter`) 1)))
    (if (== _output_get 4)
      (`/Game/Blueprints/CharacterBP/bp_baseCharacter.Damage_send` _enemy 40 2.0 (0.0 0.0 0.0) 0.0)
      (else
        (`/Game/Blueprints/CharacterBP/bp_baseCharacter.Damage_send` _enemy 40 2.0 (`self.GetActorForwardVector` _player) 3000.0)
        (`self.K2_DestroyActor`)))
    (else
      (`KismetSystemLibrary.PrintString` "NOOOOO"))))

(fn `UserConstructionScript`)