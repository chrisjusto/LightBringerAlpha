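; Player projectile that damages a target enemy and can launch it, self-destructing after five seconds.
; LaunchatEnemy stores the target and fires the physics Sphere with an impulse along the supplied vector.
; Sphere1 overlapping that target stops physics, removes health, optionally sends hitstun and player-relative launch through DamageSend, then destroys after a short delay.
; Sphere overlapping any other actor spawns a blast effect and destroys the projectile immediately.
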(event `self.ReceiveBeginPlay`
  (`KismetSystemLibrary.Delay` 5.0)
  (`self.K2_DestroyActor`))

(event `Launch`
  (params (NewParam :type "/Game/Blueprints/CharacterBP/SECONDdRAFTcHARACTER/BasePlayer_BP Object Reference") (NewParam2 :type Boolean)))

(event `self.Sphere1.OnComponentBeginOverlap`
  (params (OverlappedComponent :type "PrimitiveComponent Object Reference") (OtherActor :type "Actor Object Reference") (OtherComp :type "PrimitiveComponent Object Reference") (OtherBodyIndex :type Integer) (bFromSweep :type Boolean) (SweepResult :type "HitResult Structure (by ref)"))
  (bind _player (`self.Player`))
  (bind _launchvectorup (`self.launchVectorUp`))
  (bind _enemy (`self.Enemy`))
  (bind _returnvalue (`self.GetActorRightVector` _player))
  (if (== OtherActor _enemy)
    (`PrimitiveComponent.SetSimulatePhysics` (`self.Sphere`) false)
    (set `/Game/Blueprints/CharacterBP/bp_baseCharacter.currentHealth` (- (`/Game/Blueprints/CharacterBP/bp_baseCharacter.currentHealth` _enemy) 1) _enemy)
    (if (not (not (`self.launches?`)))
      (switch `/Game/Blueprints/enums/LaunchDirections` (`self.LaunchVector`)
        (:`NewEnumerator0`
          (`/Game/Blueprints/CharacterBP/bp_baseCharacter.Damage_send` (`self.Enemy`) 0 (`self.Hitstun`) (+ _launchvectorup (`self.GetActorForwardVector` _player)) (`self.launchDistance`)))
        (:`NewEnumerator1`
          (`/Game/Blueprints/CharacterBP/bp_baseCharacter.Damage_send` (`self.Enemy`) 0 (`self.Hitstun`) (+ _launchvectorup (* _returnvalue -1.0)) (`self.launchDistance`)))
        (:`NewEnumerator2`
          (`/Game/Blueprints/CharacterBP/bp_baseCharacter.Damage_send` (`self.Enemy`) 0 (`self.Hitstun`) (+ _launchvectorup _returnvalue) (`self.launchDistance`)))
        (:`NewEnumerator3`
          (`/Game/Blueprints/CharacterBP/bp_baseCharacter.Damage_send` (`self.Enemy`) 0 (`self.Hitstun`) (`self.launchVectorUp`) (`self.launchDistance`)))))
    (`KismetSystemLibrary.Delay` 0.5)
    (`self.DESTROY`)))

(event `self.Sphere.OnComponentBeginOverlap`
  (params (OverlappedComponent :type "PrimitiveComponent Object Reference") (OtherActor :type "Actor Object Reference") (OtherComp :type "PrimitiveComponent Object Reference") (OtherBodyIndex :type Integer) (bFromSweep :type Boolean) (SweepResult :type "HitResult Structure (by ref)"))
  (if (!= OtherActor self)
    (`KismetSystemLibrary.PrintString` "Hello")
    (`|ExecutionSequence`
      (:`then_0`
        (`/Engine/EditorBlueprintResources/StandardMacros.DoOnce` false
          (:`Completed`
            (`GameplayStatics.SpawnEmitterAtLocation` "/Game/Particles/p_blast.p_blast" (`SceneComponent.K2_GetComponentLocation` (`self.Sphere1`)) (struct) (10.0 10.0 10.0)))))
      (:`then_1`
        (`self.K2_DestroyActor`)))
    (else
      (`KismetSystemLibrary.PrintString` "no"))))

(fn `DESTROY`
  (`self.K2_DestroyActor`))

(fn `LaunchatEnemy`
  (params (P_ForwardVector :type "Vector Structure") (Player :type "/Game/Blueprints/CharacterBP/bp_baseCharacter Object Reference") (Enemey :type "/Game/Blueprints/CharacterBP/bp_baseCharacter Object Reference"))
  (set `self.Enemy` Enemey)
  (`PrimitiveComponent.AddImpulse` (`self.Sphere`) (* P_ForwardVector (`self.ProjectileSpeed`)) "None" false))

(fn `UserConstructionScript`)